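; BP_AnimatedPlatform is a platform actor that moves between its start location and a relative target offset.
; On BeginPlay it caches the start location, then plays a timeline at a configurable speed and starting progress, lerping the actor position each update without sweeping.
; When the repeat flag is set, the timeline reverses on finish to ping-pong, using events that send it toward either end.
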(event Custom|MoveToTargetLocation
  (bind (_direction _start2end) (Timeline|Timeline PlayFromStart)
    (:Update
      (CallFunction|UpdateLocation _start2end))
    (:Finished
      (if (Variables|Default|GetRepeative)
        (switch Utilities|FlowControl|Switch|SwitchonETimelineDirection _direction
          (:Forward
            (CallFunction|MovetoStartLocation))
          (:Backward
            (CallFunction|MovetoTargetLocation)))))))

(event Custom|MoveToStartLocation
  (bind (_direction _start2end) (Timeline|Timeline ReverseFromEnd)
    (:Update
      (CallFunction|UpdateLocation _start2end))
    (:Finished
      (if (Variables|Default|GetRepeative)
        (switch Utilities|FlowControl|Switch|SwitchonETimelineDirection _direction
          (:Forward
            (CallFunction|MovetoStartLocation))
          (:Backward
            (CallFunction|MovetoTargetLocation)))))))

(event EventBeginPlay
  (bind _timeline (Variables|Default|GetTimeline))
  (Variables|Default|SetStartLocation (Transformation|GetActorLocation))
  (Components|Timeline|SetPlayRate _timeline (Variables|Default|GetSpeed))
  (Components|Timeline|SetPlaybackPosition _timeline (Math|Float|Clamp(Float) (Variables|Default|GetStartProgress) 0.0 0.9999) false true)
  (bind (_direction _start2end) (Timeline|Timeline Play)
    (:Update
      (CallFunction|UpdateLocation _start2end))
    (:Finished
      (if (Variables|Default|GetRepeative)
        (switch Utilities|FlowControl|Switch|SwitchonETimelineDirection _direction
          (:Forward
            (CallFunction|MovetoStartLocation))
          (:Backward
            (CallFunction|MovetoTargetLocation)))))))

(event Collision|EventActorBeginOverlap
  (params (OtherActor :type Actor%20Object%20Reference)))

(event EventTick
  (params (DeltaSeconds :type Float%20%28single-precision%29)))

(fn ConstructionScript)

(fn UpdateLocation
  (params (Alpha :type Float%20%28single-precision%29))
  (bind _startlocation (Variables|Default|GetStartLocation))
  (Transformation|SetActorLocation (Math|Vector|Lerp(Vector) _startlocation (+ _startlocation (Variables|Default|GetTargetLocationRelative)) Alpha) false false))