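; BP_Platform_Illuminated is a Paper2D sprite platform that is solid to pawns only while a light ball overlaps it.
; Overlap begin and end events count overlapping BP-LightBall actors, enabling the platform when the count reaches one and disabling it when it returns to zero.
; Enable and disable switch the sprite's Pawn collision response between Block and Ignore and print debug messages.
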(event EventBeginPlay)

(event Collision|EventActorBeginOverlap
  (params (OtherActor :type Actor%20Object%20Reference))
  (Utilities|Casting|CastToBP-LightBall OtherActor)
  (bind _output_get (Variables|Default|SetOverlappingLightBalls (+ (Variables|Default|GetOverlappingLightBalls) 1)))
  (Math|Integer|CompareInt _output_get 1
    (:==
      (CallFunction|EnablePlatform))))

(event EventTick
  (params (DeltaSeconds :type Float%20%28single-precision%29)))

(event Collision|EventActorEndOverlap
  (params (OtherActor :type Actor%20Object%20Reference))
  (Utilities|Casting|CastToBP-LightBall OtherActor)
  (bind _output_get (Variables|Default|SetOverlappingLightBalls (+ (Variables|Default|GetOverlappingLightBalls) -1)))
  (Math|Integer|CompareInt _output_get 0
    (:==
      (CallFunction|DisablePlatform))))

(fn ConstructionScript)

(fn EnablePlatform
  (Collision|SetCollisionResponsetoChannel (Variables|Default|GetPaperSprite) "ECC_Pawn" "ECR_Block")
  (Development|PrintString "Platform Enabled!"))

(fn DisablePlatform
  (Collision|SetCollisionResponsetoChannel (Variables|Default|GetPaperSprite) "ECC_Pawn" "ECR_Ignore")
  (Development|PrintString "Platform Disabled!"))