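; Elevator lever that sends its linked Platform to the target or back to the start when a boomerang overlaps it.
; Hits are ignored while the platform's timeline plays; otherwise its playback position decides the direction.
; The lever binds to the platform's move events to swing LeverRoot's pitch with its own Timeline.
; BeginPlay copies the platform timeline's play rate and sets initial tilt from StartProgress.
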(event Custom|LeverToStartEvent
  (bind _newtrack_1 (Timeline|Timeline ReverseFromEnd)
    (:Update
      (Transformation|SetRelativeRotation (Variables|Default|GetLeverRoot) (Math|Rotator|MakeRotator 0.0 (* _newtrack_1 (Variables|Default|GetRotationVal)) 0.0) false false))))

(event Custom|LeverToTargetEvent
  (bind _newtrack_1 (Timeline|Timeline PlayFromStart)
    (:Update
      (Transformation|SetRelativeRotation (Variables|Default|GetLeverRoot) (Math|Rotator|MakeRotator 0.0 (* _newtrack_1 (Variables|Default|GetRotationVal)) 0.0) false false))))

(event EventBeginPlay
  (bind _platform (Variables|Default|GetPlatform))
  (Components|Timeline|SetPlayRate (Variables|Default|GetTimeline) (Components|Animation|GetPlayRate (Variables|/Game/Classes/BP_AnimatedPlatform.BP_AnimatedPlatform_C|GetTimeline (Variables|Default|GetPlatform))))
  (Transformation|SetRelativeRotation (Variables|Default|GetLeverRoot) (Math|Rotator|MakeRotator 0.0 (* (- (* (Variables|/Game/Classes/BP_AnimatedPlatform.BP_AnimatedPlatform_C|GetStartProgress (Variables|Default|GetPlatform)) 2.0) 1.0) (Variables|Default|GetRotationVal)) 0.0) false false)
  (EventDispatchers|BindEventtoMovetoStart _platform (delegate Custom|LeverToStartEvent))
  (EventDispatchers|BindEventtoMovetoTarget _platform (delegate Custom|LeverToTargetEvent)))

(event Collision|EventActorBeginOverlap
  (params (OtherActor :type Actor%20Object%20Reference))
  (bind _platform (Variables|Default|GetPlatform))
  (bind _platform_2 (Variables|Default|GetPlatform))
  (bind _timeline (Variables|/Game/Classes/BP_AnimatedPlatform.BP_AnimatedPlatform_C|GetTimeline _platform))
  (Utilities|Casting|CastToBP-Boomerang OtherActor)
  (if (not (Audio|Components|Audio|IsPlaying _timeline))
    (Math|Float|CompareFloat (Components|Timeline|GetPlaybackPosition _timeline) 0.001
      (:>
        (Default|CallMovetoStart _platform_2))
      (:==
        (Default|CallMovetoTarget _platform_2 :!label _label))
      (:<
        (goto _label)))))

(event EventTick
  (params (DeltaSeconds :type Float%20%28single-precision%29)))

(fn ConstructionScript)